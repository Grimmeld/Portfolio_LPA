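; BP_Banc is an interactable that opens a project information screen for the player, with a Losange component rotating every tick.
; Interact creates a project display widget from its title, description and paragraphs, plays its appear animation, and hides the object's own Widget component.
; It also passes its Torch to the controller as the current torch.
; Interacting again removes the display through the controller and shows the Widget again.
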(event EventTick
  (params (DeltaSeconds :type Float%20%28single-precision%29))
  (Transformation|AddWorldRotation (Variables|Default|GetLosange) (Math|Rotator|MakeRotator 0.0 0.0 (Variables|Anim|GetRotateSpeed)) false false))

(event EventInteract
  (bind _player_ref (Variables|Default|GetPlayer_Ref))
  (bind _controllerref (Variables|/Game/TopDown/Blueprints/BP_TopDownCharacter.BP_TopDownCharacter_C|GetControllerRef _player_ref))
  (if (Variables|/Game/TopDown/Blueprints/BP_TopDownController.BP_TopDownController_C|GetisInteracting _controllerref)
    (Default|RemoveWidgetProject _controllerref)
    (Development|SetHiddeninGame (Variables|Default|GetWidget) false false)
    (else
      (bind _output_get (Variables|/Game/TopDown/Blueprints/BP_TopDownController.BP_TopDownController_C|SetisInteracting _controllerref true))
      (Development|SetHiddeninGame (Variables|Default|GetWidget) _output_get false)
      (Utilities|FlowControl|Sequence
        (:then_0
          ;[0.15 0.15 0.15 0.5] Widget
          (bind _returnvalue (UserInterface|CreateWidget "/Game/Blueprint/UI/WBP_ProjectDisplay.WBP_ProjectDisplay_C" _controllerref (Variables|Project|GetTitle) (Variables|Project|GetInfo) (Variables|Project|GetParagraphes)))
          (Default|SetWidgetProject _controllerref _returnvalue)
          (UserInterface|Viewport|AddtoViewport _returnvalue 0))
        (:then_1
          (Default|PlayAppear (Variables|/Game/TopDown/Blueprints/BP_TopDownController.BP_TopDownController_C|GetWidgetProject _controllerref) "Forward"))
        (:then_2
          (Variables|/Game/TopDown/Blueprints/BP_TopDownController.BP_TopDownController_C|SetCurrentTorch (Variables|/Game/TopDown/Blueprints/BP_TopDownCharacter.BP_TopDownCharacter_C|GetControllerRef (Variables|Default|GetPlayer_Ref)) (Variables|Progression|GetTorch)))))))

(fn ConstructionScript
  (|CallParentFunction))