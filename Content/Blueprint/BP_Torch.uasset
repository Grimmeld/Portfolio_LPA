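; BP_Torch is a torch actor that can be lit at runtime through its LightFire event.
; It caches the point light's starting intensity on BeginPlay.
; LightFire flags the torch as lit, reveals the fire after a short delay, then plays a timeline that scales both the fire and the light intensity by the same factor.
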(event Custom|LightFire
  (Variables|Default|SetIsLightened true)
  (Utilities|FlowControl|Delay 0.2)
  (Development|SetHiddeninGame (Variables|Default|GetFire) false true)
  (bind _factor (Timeline|ScaleFire Play)
    (:Update
      (Transformation|SetWorldScale3D (Variables|Default|GetFire) (Math|Vector|MakeVector _factor _factor _factor))
      (Rendering|Components|Light|SetIntensity (Variables|Default|GetPointLight) (* _factor (Variables|Default|GetIntensity))))))

(event EventBeginPlay
  (Variables|Default|SetIntensity (Variables|/Script/Engine.LightComponentBase|GetIntensity (Variables|Default|GetPointLight))))

(fn ConstructionScript)