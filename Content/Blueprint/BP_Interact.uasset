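; BP_Interact is an interactable actor with an empty Interact event and two proximity prompts that turn toward the player's camera every Tick.
; Trigger_Far plays the far widget's appear and disappear animations.
; Trigger_Interact swaps the far prompt for the near one and sets or clears this actor as the player's interactable.
; Clicking the mesh calls Interact whenever the player has any valid interactable, without checking it is this actor.
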(event OnComponentBeginOverlap(Trigger_Interact)
  (params (OverlappedComponent :type Primitive%20Component%20Object%20Reference) (OtherActor :type Actor%20Object%20Reference) (OtherComp :type Primitive%20Component%20Object%20Reference) (OtherBodyIndex :type Integer) (bFromSweep :type Boolean) (SweepResult :type Hit%20Result%20Structure%20%28by%20ref%29))
  (if (== OtherActor (Variables|Default|GetPlayer_Ref))
    (Development|SetHiddeninGame (Variables|Default|GetWidget) false false)
    (Development|SetHiddeninGame (Variables|Default|GetWidgetFar) true false)
    (Default|Disappear (Variables|Default|GetWidgetFar_Ref))
    (Default|SetInterable (Variables|Default|GetPlayer_Ref) self)))

(event OnComponentEndOverlap(Trigger_Interact)
  (params (OverlappedComponent :type Primitive%20Component%20Object%20Reference) (OtherActor :type Actor%20Object%20Reference) (OtherComp :type Primitive%20Component%20Object%20Reference) (OtherBodyIndex :type Integer))
  (if (== OtherActor (Variables|Default|GetPlayer_Ref))
    (Development|SetHiddeninGame (Variables|Default|GetWidget) true false)
    (Development|SetHiddeninGame (Variables|Default|GetWidgetFar) false false)
    (Default|PlayAppear (Variables|Default|GetWidgetFar_Ref))
    (Default|SetInterable (Variables|Default|GetPlayer_Ref))))

(event OnClicked(Mesh)
  (params (TouchedComponent :type Primitive%20Component%20Object%20Reference) (ButtonPressed :type Key%20Structure :default "None"))
  ;[0.15 0.15 0.15 0.5] Interact with clic
  (if (Utilities|IsValid (Variables|/Game/TopDown/Blueprints/BP_TopDownCharacter.BP_TopDownCharacter_C|GetInteractable (Variables|Default|GetPlayer_Ref)))
    (CallFunction|Interact)))

(event OnComponentBeginOverlap(Trigger_Far)
  (params (OverlappedComponent :type Primitive%20Component%20Object%20Reference) (OtherActor :type Actor%20Object%20Reference) (OtherComp :type Primitive%20Component%20Object%20Reference) (OtherBodyIndex :type Integer) (bFromSweep :type Boolean) (SweepResult :type Hit%20Result%20Structure%20%28by%20ref%29))
  (if (== OtherActor (Variables|Default|GetPlayer_Ref))
    (Default|PlayAppear (Variables|Default|GetWidgetFar_Ref))))

(event OnComponentEndOverlap(Trigger_Far)
  (params (OverlappedComponent :type Primitive%20Component%20Object%20Reference) (OtherActor :type Actor%20Object%20Reference) (OtherComp :type Primitive%20Component%20Object%20Reference) (OtherBodyIndex :type Integer))
  (if (== OtherActor (Variables|Default|GetPlayer_Ref))
    (Default|Disappear (Variables|Default|GetWidgetFar_Ref))))

(event Custom|Interact)

(event EventBeginPlay
  (bind _asbp_top_down_character (Utilities|Casting|CastToBP_TopDownCharacter (Game|GetPlayerCharacter 0)))
  (Variables|Default|SetPlayer_Ref _asbp_top_down_character)
  (Development|SetHiddeninGame (Variables|Default|GetWidget) true false)
  (bind _aswbp_interact_far (Utilities|Casting|CastToWBP_InteractFar (UserInterface|GetWidget (Variables|Default|GetWidgetFar))))
  (Variables|Default|SetWidgetFar_Ref _aswbp_interact_far))

(event EventTick
  (params (DeltaSeconds :type Float%20%28single-precision%29))
  (bind _player_ref (Variables|Default|GetPlayer_Ref))
  (bind _widget (Variables|Default|GetWidget))
  (bind _widgetfar (Variables|Default|GetWidgetFar))
  (bind _camera (Variables|/Game/TopDown/Blueprints/BP_TopDownCharacter.BP_TopDownCharacter_C|GetCamera _player_ref))
  (bind _returnvalue (Transformation|GetWorldLocation _camera))
  (Utilities|FlowControl|Sequence
    (:then_0
      (if (Utilities|IsValid _player_ref)
        (Transformation|SetWorldRotation _widget (Math|Rotator|FindLookatRotation (Transformation|GetWorldLocation _widget) _returnvalue) false false)
        (Transformation|SetWorldRotation _widgetfar (Math|Rotator|FindLookatRotation (Transformation|GetWorldLocation _widgetfar) _returnvalue) false false)))))

(fn ConstructionScript)